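; Game mode Blueprint that shuts down enemy grunt AI when the player dies.
; On BeginPlay it casts the player character to BP_ShadowFig and binds to its OnPlayerDeath event.
; On death it loops over every AIC_Grunt controller, clearing focus, stopping movement, disabling sight perception and resetting the player-related Blackboard flags to false.
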(event `self.ReceiveBeginPlay`
  (bind _asbp_shadow_fig (cast `/Game/Game/Blueprints/BP_ShadowFig` (`GameplayStatics.GetPlayerCharacter` 0)))
  (bind _output_get (set `self.PlayerRef` _asbp_shadow_fig))
  (add `/Game/Game/Blueprints/BP_ShadowFig.OnPlayerDeath` _output_get (delegate `OnPlayerDied`)))

(event `OnPlayerDied`
  (bind _outactors (`GameplayStatics.GetAllActorsOfClass` "/Game/Game/Blueprints/NPC_AI/AIC_Grunt.AIC_Grunt_C"))
  (for _array_element _outactors
    (bind _blackboard (`AIController.Blackboard` _array_element))
    (`BlackboardComponent.SetValueAsBool` _blackboard "PlayerAlive" false)
    (`AIController.K2_ClearFocus` _array_element)
    (`Controller.StopMovement` _array_element)
    (`AIPerceptionComponent.SetSenseEnabled` (`AIController.GetAIPerceptionComponent` _array_element) "/Script/AIModule.AISense_Sight" false)
    (`BlackboardComponent.SetValueAsBool` _blackboard "IsNearPlayer" false)
    (`BlackboardComponent.SetValueAsBool` _blackboard "IsDetected" false)))

(fn `UserConstructionScript`)