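; AI controller for the masked Grunt NPC that runs BT_Grunt, seeding its blackboard with the next nav-point destination from a looping list.
; Perception events flag actors with the target tag as detected, and Tick flags whether that actor is near.
; Tick also switches walk speed and gun pose between detected and undetected states.
; A sight viewpoint override takes location and rotation from the mesh's eyes socket.
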(event `self.ReceiveBeginPlay`
  (bind _asbp_mask_grunt (cast `/Game/Game/Blueprints/NPC_AI/BP_MaskGrunt` (`self.K2_GetPawn`)))
  (set `self.As BP Mask Grunt` _asbp_mask_grunt)
  (`self.RunBehaviorTree` "/Game/Game/Blueprints/NPC_AI/BT_Grunt.BT_Grunt")
  (bind _destination (`self.Get Next Destination`))
  (`self.SetNextDestination` _destination))

(event `self.AIPerception.OnTargetPerceptionUpdated`
  (params (Actor :type "Actor Object Reference") (Stimulus :type "AIStimulus Structure"))
  (bind (_age _expirationage _strength _stimuluslocation _receiverlocation _tag _bsuccessfullysensed) (break `AIStimulus` Stimulus))
  ;[1 0.125 0.125] AI Perception
  (if (== (`|GetArrayItem` (`Actor.Tags` Actor)) (`self.TagTarget`))
    (set `self.Sensed` _bsuccessfullysensed)
    (set `self.PlayerRef` Actor)
    (`BlackboardComponent.SetValueAsBool` (`self.Blackboard`) "IsDetected" _bsuccessfullysensed)))

(event `self.ReceiveTick`
  (params (DeltaSeconds :type "Float (single-precision)"))
  (bind _as_bp_mask_grunt (`self.As BP Mask Grunt`))
  (bind _charactermovement (`Character.CharacterMovement` _as_bp_mask_grunt))
  (bind _gruntgun (`/Game/Game/Blueprints/NPC_AI/BP_MaskGrunt.GruntGun` _as_bp_mask_grunt))
  (bind _gruntgun_2 (`/Game/Game/Blueprints/NPC_AI/BP_MaskGrunt.GruntGun` _as_bp_mask_grunt))
  (bind (_returnvalue_location _returnvalue_rotation _returnvalue_scale) (`KismetMathLibrary.BreakTransform` (`SceneComponent.GetRelativeTransform` _gruntgun)))
  (bind (_returnvalue_location_2 _returnvalue_rotation_2 _returnvalue_scale_2) (`KismetMathLibrary.BreakTransform` (`SceneComponent.GetRelativeTransform` _gruntgun_2)))
  (bind (_returnvalue_location_3 _returnvalue_rotation_3 _returnvalue_scale_3) (`KismetMathLibrary.BreakTransform` (`KismetMathLibrary.MakeTransform` (-38.3 -10.2 5.9) (struct :`Pitch` 0.45 :`Yaw` -94.0 :`Roll` -142.0) _returnvalue_scale)))
  (bind (_returnvalue_location_4 _returnvalue_rotation_4 _returnvalue_scale_4) (`KismetMathLibrary.BreakTransform` (`KismetMathLibrary.MakeTransform` (-48.5 -6.1 -1.4) (struct :`Pitch` 0.45 :`Yaw` -94.0 :`Roll` -176.9) _returnvalue_scale_2)))
  ;[1 1 1] Vérifier si le joueur est proche
  (`|ExecutionSequence`
    (:`then_0`
      (if (`self.Sensed`)
        (`BlackboardComponent.SetValueAsBool` (`self.Blackboard`) "IsNearPlayer" (<= (`KismetMathLibrary.VSize` (- (`self.K2_GetActorLocation` (`self.PlayerRef`)) (`self.K2_GetActorLocation` (`self.As BP Mask Grunt`)))) (`self.NearDetection`)))))
    (:`then_1`
      ;[1 1 1] Aiming Or Not
      (if (`BlackboardComponent.GetValueAsBool` (`self.Blackboard`) "IsDetected")
        (set `CharacterMovementComponent.MaxWalkSpeed` 100.0 _charactermovement)
        (`SceneComponent.K2_SetRelativeTransform` _gruntgun (`KismetMathLibrary.MakeTransform` _returnvalue_location_3 _returnvalue_rotation_3 _returnvalue_scale_3) false false)
        (else
          (set `CharacterMovementComponent.MaxWalkSpeed` 150.0 _charactermovement)
          (`SceneComponent.K2_SetRelativeTransform` _gruntgun_2 (`KismetMathLibrary.MakeTransform` _returnvalue_location_4 _returnvalue_rotation_4 _returnvalue_scale_4) false false))))))

(event `self.AIPerception.OnTargetPerceptionForgotten`
  (params (Actor :type "Actor Object Reference"))
  ;[1 0.125 0.125] AI Perception
  (if (== (`|GetArrayItem` (`Actor.Tags` Actor)) (`self.TagTarget`))
    (`BlackboardComponent.SetValueAsBool` (`self.Blackboard`) "IsDetected" false)))

(fn `DetermineAISightPerceptionViewPoint`
  (returns (OutLocation :type "Vector Structure") (OutRotation :type "Rotator Structure"))
  (bind _asbp_mask_grunt (cast `/Game/Game/Blueprints/NPC_AI/BP_MaskGrunt` (`self.K2_GetPawn`)))
  (bind (_returnvalue_location _returnvalue_rotation) (`KismetMathLibrary.BreakTransform` (`SceneComponent.GetSocketTransform` (`Character.Mesh` _asbp_mask_grunt) "eyes_socket" "RTS_World")))
  (return _returnvalue_location _returnvalue_rotation))

(fn `Get Next Destination`
  (returns (Destination :type "Vector Structure"))
  (bind _navpoints (`/Game/Game/Blueprints/NPC_AI/BP_MaskGrunt.NavPoints` (`self.As BP Mask Grunt`)))
  (bind _output_get (set `self.ActualNavPointIndex` (+ (`self.ActualNavPointIndex`) 1)))
  (return (`self.K2_GetActorLocation` (`|GetArrayItem` _navpoints (mod _output_get (`KismetArrayLibrary.Array_Length` _navpoints))))))

(fn `SetNextDestination`
  (params (Destination :type "Vector Structure"))
  (`BlackboardComponent.SetValueAsVector` (`self.Blackboard`) "NextDestination" Destination))

(fn `UserConstructionScript`)